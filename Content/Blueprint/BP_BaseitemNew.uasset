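; Base item actor that shows proximity icons as the player character approaches it.
; An outer sphere overlap shows a distant icon, and an inner sphere overlap swaps it for a close-range icon, reversing on exit.
; The construction script applies configurable sphere radii, mesh, mesh scale and icon location, with a debug flag setting inner icon visibility.
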(event `self.InnerSphere.OnComponentBeginOverlap`
  (params (OverlappedComponent :type "PrimitiveComponent Object Reference") (OtherActor :type "Actor Object Reference") (OtherComp :type "PrimitiveComponent Object Reference") (OtherBodyIndex :type Integer) (bFromSweep :type Boolean) (SweepResult :type "HitResult Structure (by ref)"))
  (if (== OtherActor (`GameplayStatics.GetPlayerCharacter` 0))
    (`SceneComponent.SetVisibility` (`self.InnerSphereIcon`) true false)
    (`SceneComponent.SetVisibility` (`self.OuterSphereIcon`) false false)))

(event `self.InnerSphere.OnComponentEndOverlap`
  (params (OverlappedComponent :type "PrimitiveComponent Object Reference") (OtherActor :type "Actor Object Reference") (OtherComp :type "PrimitiveComponent Object Reference") (OtherBodyIndex :type Integer))
  (if (== (`GameplayStatics.GetPlayerCharacter` 0) OtherActor)
    (`SceneComponent.SetVisibility` (`self.InnerSphereIcon`) false false)
    (`SceneComponent.SetVisibility` (`self.OuterSphereIcon`) true false)))

(event `self.OuterSphere.OnComponentBeginOverlap`
  (params (OverlappedComponent :type "PrimitiveComponent Object Reference") (OtherActor :type "Actor Object Reference") (OtherComp :type "PrimitiveComponent Object Reference") (OtherBodyIndex :type Integer) (bFromSweep :type Boolean) (SweepResult :type "HitResult Structure (by ref)"))
  (if (== OtherActor (`GameplayStatics.GetPlayerCharacter` 0))
    (`SceneComponent.SetVisibility` (`self.OuterSphereIcon`) true false)))

(event `self.OuterSphere.OnComponentEndOverlap`
  (params (OverlappedComponent :type "PrimitiveComponent Object Reference") (OtherActor :type "Actor Object Reference") (OtherComp :type "PrimitiveComponent Object Reference") (OtherBodyIndex :type Integer))
  (if (== (`GameplayStatics.GetPlayerCharacter` 0) OtherActor)
    (`SceneComponent.SetVisibility` (`self.OuterSphereIcon`) false false)))

(fn `UserConstructionScript`
  (bind _innersphereicon (`self.InnerSphereIcon`))
  (bind _staticmesh (`self.StaticMesh`))
  (`|ExecutionSequence`
    (:`then_0`
      (`SphereComponent.SetSphereRadius` (`self.InnerSphere`) (`self.Inner Sphere Radius`) true)
      (`SphereComponent.SetSphereRadius` (`self.OuterSphere`) (`self.outer Sphere Radius`) true))
    (:`then_1`
      (`StaticMeshComponent.SetStaticMesh` _staticmesh (`self.Mesh`))
      (`SceneComponent.K2_SetWorldTransform` _staticmesh (`KismetMathLibrary.MakeTransform` (`SceneComponent.K2_GetComponentLocation` _staticmesh) (`SceneComponent.K2_GetComponentRotation` _staticmesh) (`self.Mesh Scale`)) false false))
    (:`then_2`
      (`SceneComponent.K2_SetRelativeLocation` _innersphereicon (`self.Icon Location`) false false)
      (`SceneComponent.K2_SetRelativeLocation` (`self.OuterSphereIcon`) (`self.Icon Location`) false false)
      (`SceneComponent.SetVisibility` _innersphereicon (`self.DebugMode`) false))))