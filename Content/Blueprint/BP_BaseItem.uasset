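; BP_BaseItem is an item Blueprint that shows proximity icons to the local player character.
; Overlap events on InnerSphere swap visibility between the inner and outer icons as player character 0 enters or leaves.
; The outer icon's show and hide events are bound to the OuterSphereIcon component itself rather than to OuterSphere.
; The construction script sizes both spheres from radius variables.
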(event `self.InnerSphere.OnComponentBeginOverlap`
  (params (OverlappedComponent :type "PrimitiveComponent Object Reference") (OtherActor :type "Actor Object Reference") (OtherComp :type "PrimitiveComponent Object Reference") (OtherBodyIndex :type Integer) (bFromSweep :type Boolean) (SweepResult :type "HitResult Structure (by ref)"))
  (if (== OtherActor (`GameplayStatics.GetPlayerCharacter` 0))
    (`SceneComponent.SetVisibility` (`self.InnerSphereIcon`) true false)
    (`SceneComponent.SetVisibility` (`self.OuterSphereIcon`) false false)))

(event `self.InnerSphere.OnComponentEndOverlap`
  (params (OverlappedComponent :type "PrimitiveComponent Object Reference") (OtherActor :type "Actor Object Reference") (OtherComp :type "PrimitiveComponent Object Reference") (OtherBodyIndex :type Integer))
  (if (== (`GameplayStatics.GetPlayerCharacter` 0) OtherActor)
    (`SceneComponent.SetVisibility` (`self.InnerSphereIcon`) false false)
    (`SceneComponent.SetVisibility` (`self.OuterSphereIcon`) true false)))

(event `self.OuterSphereIcon.OnComponentBeginOverlap`
  (params (OverlappedComponent :type "PrimitiveComponent Object Reference") (OtherActor :type "Actor Object Reference") (OtherComp :type "PrimitiveComponent Object Reference") (OtherBodyIndex :type Integer) (bFromSweep :type Boolean) (SweepResult :type "HitResult Structure (by ref)"))
  (if (== OtherActor (`GameplayStatics.GetPlayerCharacter` 0))
    (`SceneComponent.SetVisibility` (`self.OuterSphereIcon`) true false)))

(event `self.OuterSphereIcon.OnComponentEndOverlap`
  (params (OverlappedComponent :type "PrimitiveComponent Object Reference") (OtherActor :type "Actor Object Reference") (OtherComp :type "PrimitiveComponent Object Reference") (OtherBodyIndex :type Integer))
  (if (== (`GameplayStatics.GetPlayerCharacter` 0) OtherActor)
    (`SceneComponent.SetVisibility` (`self.OuterSphereIcon`) false false)))

(fn `UserConstructionScript`
  (`SphereComponent.SetSphereRadius` (`self.InnerSphere`) (`self.In Sphere Radius`) true)
  (`SphereComponent.SetSphereRadius` (`self.OuterSphere`) (`self.Outer Sphere Radius`) true))