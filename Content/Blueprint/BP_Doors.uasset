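; BP_Doors is an interactable door that swings open and closed.
; Its Interact event flips the open state and plays or reverses a timeline, whose alpha lerps the door mesh's relative yaw between closed and 100 degrees.
; An IsMoving flag ignores further interactions until the timeline finishes.
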(event `/Game/FirstPerson/Blueprints/Interface/I_Interact.Interact`
  (if (not (`self.IsMoving`))
    (set `self.IsMoving` true)
    (bind _output_get (set `self.IsOpened` (not (`self.IsOpened`))))
    (if _output_get
      (bind (_direction _alpha_doors) (`Timeline|TL_Doors` :!label _label)
        (:`Update`
          (`SceneComponent.K2_SetRelativeRotation` (`self.Sm_Door`) (`KismetMathLibrary.MakeRotator` 0.0 0.0 (`KismetMathLibrary.Lerp` 0.0 100.0 _alpha_doors)) false false))
        (:`Finished`
          (set `self.IsMoving` false)))
      (else
        (goto _label :!via `Reverse`)))))

(fn `UserConstructionScript`)